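; BP_GI_Base is a Game Instance Blueprint that handles hosting and joining LAN multiplayer sessions.
; CreateGame creates a LAN session, then on success hides the mouse cursor and opens M_Play_1 as a listen server, with debug prints along the way.
; FindGame searches for a single LAN session and joins the first result, with no failure handling.
; Reconnect waits briefly, then reuses the FindGame search-and-join path.
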(event Custom|CreateGame
  (Development|PrintString "222")
  (|Session (Game|GetPlayerController 0) 10 true
    (:then
      (Development|PrintString "111"))
    (:OnSuccess
      (Variables|/Script/Engine.PlayerController|SetbShowMouseCursor (Game|GetPlayerController 0) false)
      (Game|OpenLevel(byName) "M_Play_1" true "listen")
      (Development|PrintString "Create"))
    (:OnFailure
      (Development|PrintString "Fail"))))

(event Custom|FindGame
  (bind _results (|FindSessions (Game|GetPlayerController 0) 1 true)
    (:OnSuccess
      (|JoinSession (Game|GetPlayerController 0) (Utilities|Array|Get(acopy) _results)))))

(event Custom|Reconnect
  (Utilities|FlowControl|Delay 1.0)
  (bind _results (|FindSessions (Game|GetPlayerController 0) 1 true)
    (:OnSuccess
      (|JoinSession (Game|GetPlayerController 0) (Utilities|Array|Get(acopy) _results)))))