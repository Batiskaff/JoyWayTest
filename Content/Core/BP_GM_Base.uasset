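; BP_GM_Base is a game mode Blueprint that handles player joins and spawns characters for every player after the first.
; On PostLogin it adds each BP_PC_Base controller to the AllPC array, skipping spawn logic while that array holds only one.
; For later joins, it spawns a FirstPersonCharacter at the BP_A_Respawn actor matching the controller's array index, then possesses it.
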(event EventPostLogin
  (params (NewPlayer :type Player%20Controller%20Object%20Reference))
  (bind _all_pc (Variables|Default|GetAll_PC))
  (bind _asbp_pc_base (Utilities|Casting|CastToBP_PC_Base NewPlayer))
  (bind _returnvalue (Utilities|Array|Add _all_pc _asbp_pc_base))
  (if (not (== (Utilities|Array|Length _all_pc) 1))
    (bind _outactors (Actor|GetAllActorsOfClass "/Game/Core/Respawn/BP_A_Respawn.BP_A_Respawn_C"))
    (bind _returnvalue_2 (Game|SpawnActorfromClass "/Game/Core/FirstPersonCharacter.FirstPersonCharacter_C" (Math|Transform|MakeTransform (Transformation|GetActorLocation (Utilities|Array|Get(acopy) _outactors _returnvalue)) "0, 0, 0" "1,1,1") "AlwaysSpawn" 0 0))
    (Pawn|Possess _asbp_pc_base _returnvalue_2)))

(fn ConstructionScript)