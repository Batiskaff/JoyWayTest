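; BP_PC_Base is a base player controller that relays reconnect, map switch and gun spawn requests.
; ConnectAgain calls Reconnect on BP_GI_Base.
; Request events forward to matching Server-named events, which act on the first BP_A_Switcher or BP_A_GunSpawner found in the world.
; Those lookups use GetAllActorsOfClass with no check for an empty result.
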(event Custom|SwitchMapRequest
  (params (MapName :type String))
  (CallFunction|SwitchMapServer MapName))

(event Custom|ConnectAgain
  (bind _asbp_gi_base (Utilities|Casting|CastToBP_GI_Base (Game|GetGameInstance)))
  (Default|Reconnect _asbp_gi_base))

(event Custom|SwitchMapServer
  (params (map :type String))
  (bind _outactors (Actor|GetAllActorsOfClass "/Game/Core/BP_A_Switcher.BP_A_Switcher_C"))
  (Default|SwitchMap (Utilities|Array|Get(acopy) _outactors) map))

(event Custom|SpawnGunRequest
  (CallFunction|SpawnGunServer))

(event Custom|SpawnGunServer
  (bind _outactors (Actor|GetAllActorsOfClass "/Game/Core/Guns/BP_A_GunSpawner.BP_A_GunSpawner_C"))
  (Default|SpawnGun (Utilities|Array|Get(acopy) _outactors)))

(fn ConstructionScript)