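; Master gun actor that players equip, fire and drop, toggling box physics on pickup and release.
; On BeginPlay the server loads stats from DT_Gun by GunID, while clients tint the mesh through a dynamic material.
; FireStart spawns projectiles along the owner's camera, using delays for fire rate and automatic clip reload, and re-calls itself for automatic shot types.
; ReloadUI pushes ammo and timer state to a reload widget on non-server instances.
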(event Custom|Equip
  (params (bEquip :type Boolean) (Target :type Actor%20Object%20Reference))
  (bind _box (Variables|Default|GetBox))
  (if bEquip
    (bind _asfirst_person_character (Utilities|Casting|CastToFirstPersonCharacter Target))
    (Variables|Default|SetParentPawn _asfirst_person_character)
    (Physics|SetSimulatePhysics _box false)
    (Collision|SetCollisionEnabled _box "NoCollision")
    (else
      (Collision|SetCollisionEnabled _box "QueryAndPhysics")
      (Physics|SetSimulatePhysics _box true)
      (Transformation|DetachFromActor Target "KeepWorld" "KeepWorld" "KeepWorld"))))

(event Custom|ReloadUI
  (params (Reload :type Boolean) (CurrentAmmo :type Integer) (MaxAmmo :type Integer) (TimerReload :type Float%20%28single-precision%29))
  (if (not (Networking|IsServer))
    (bind _asw_gun_reload (Utilities|Casting|CastToW_Gun_Reload (UserInterface|GetUserWidgetObject (Variables|Default|GetW_ReloadGun))))
    (Default|UpdateText _asw_gun_reload Reload CurrentAmmo MaxAmmo TimerReload)))

(event EventBeginPlay
  (if (Networking|IsServer)
    (bind _returnvalue (Utilities|GetDataTableRow "/Game/Core/DT/DT_Gun.DT_Gun" (Utilities|String|StringToName (Utilities|String|ToString(Integer) (Variables|Default|GetGunID))))
      (:then
        (Variables|GunParam|SetstrGun _returnvalue)
        (Variables|GunParam|SetCurrentAmmo (Utilities|Struct|BreakSTR_Gun _returnvalue))))
    (else
      (bind _returnvalue_2 (Rendering|Material|CreateDynamicMaterialInstance "/Game/FirstPerson/FPWeapon/Materials/M_FPGun.M_FPGun" "None" :!class /Script/Engine.KismetMaterialLibrary))
      (bind _output_get (Variables|Default|SetGunDMI _returnvalue_2))
      (Rendering|Material|SetVectorParameterValue _output_get "BodyColor" (Utilities|Select :Index (Variables|Default|GetGunID) :Option%200 "(R=0.037317,G=0.129637,B=1.000000,A=1.000000)" :Option%201 "(R=0.000000,G=1.000000,B=0.962717,A=1.000000)" :Option%202 "(R=1.000000,G=0.000000,B=0.837795,A=1.000000)" :Option%203 "(R=1.000000,G=0.879726,B=0.000000,A=1.000000)") :!class /Script/Engine.MaterialInstanceDynamic)
      (Rendering|Material|SetMaterial (Variables|Default|GetSkeletalMesh) 0 _output_get))))

(event Collision|EventActorBeginOverlap
  (params (OtherActor :type Actor%20Object%20Reference)))

(event Custom|FireStop
  (Variables|Default|SetbFire false))

(event Custom|FireStart
  (bind _strgun (Variables|GunParam|GetstrGun))
  (bind _strgun_2 (Variables|GunParam|GetstrGun))
  (bind (_ammoclip _reloadammoclip) (Utilities|Struct|BreakSTR_Gun _strgun))
  (bind (_ammoclip_2 _attackspeed) (Utilities|Struct|BreakSTR_Gun _strgun_2))
  (bind _returnvalue (/ 6e+01 _attackspeed))
  (Variables|Default|SetbFire true)
  (if (and (Variables|GunParam|GetReloadAmmo) (Variables|GunParam|GetReloadClip))
    (Game|SpawnActorfromClass (Utilities|Struct|BreakSTR_Gun (Variables|GunParam|GetstrGun)) (Math|Transform|MakeTransform (Transformation|GetWorldLocation (Variables|Default|GetSpawn_Place)) (Transformation|GetWorldRotation (Variables|/Game/Core/FirstPersonCharacter.FirstPersonCharacter_C|GetFirstPersonCamera (Variables|Default|GetParentPawn)))) "AlwaysSpawn" 0 self 0) ; Spawn projectile
    (Math|Integer|DecrementInt (Variables|GunParam|GetCurrentAmmo)
      (:%20%20
        (if (== (Variables|GunParam|GetCurrentAmmo) 0)
          (Variables|GunParam|SetReloadClip false)
          (CallFunction|ReloadUI true (Variables|GunParam|GetCurrentAmmo) _ammoclip _reloadammoclip)
          (Utilities|FlowControl|Delay (.ReloadAmmoClip (Utilities|Struct|BreakSTR_Gun (Variables|GunParam|GetstrGun))))
          (Variables|GunParam|SetReloadClip true)
          (Variables|GunParam|SetCurrentAmmo (Utilities|Struct|BreakSTR_Gun (Variables|GunParam|GetstrGun)))
          (CallFunction|ReloadUI false (Variables|GunParam|GetCurrentAmmo) (Utilities|Struct|BreakSTR_Gun (Variables|GunParam|GetstrGun)) 0.0)
          (else
            (Variables|GunParam|SetReloadAmmo false)
            (CallFunction|ReloadUI true (Variables|GunParam|GetCurrentAmmo) _ammoclip_2 _returnvalue)
            (Utilities|FlowControl|Delay _returnvalue)
            (Variables|GunParam|SetReloadAmmo true)
            (CallFunction|ReloadUI false (Variables|GunParam|GetCurrentAmmo) (.AmmoClip (Utilities|Struct|BreakSTR_Gun (Variables|GunParam|GetstrGun))) 0.0)
            (if (== (Utilities|Struct|BreakSTR_Gun (Variables|GunParam|GetstrGun)) 1)
              (if (Variables|Default|GetbFire)
                (CallFunction|FireStart)))))))))

(fn ConstructionScript)